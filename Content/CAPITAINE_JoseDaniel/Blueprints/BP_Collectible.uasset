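; BP_Collectible is a pickup that adds its ScoreValue to the player's score when a BP_ThirdPersonCharacter overlaps it.
; On overlap it increments the character's Score and destroys itself.
; It then finds all top-level WBP_Score widgets and writes the new total into their DisplayText directly, rather than through a binding or event dispatcher.
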(event Collision|EventActorBeginOverlap
  (params (OtherActor :type Actor%20Object%20Reference))
  (bind _asbp_third_person_character (Utilities|Casting|CastToBP_ThirdPersonCharacter OtherActor))
  (bind _output_get (Variables|/Game/CAPITAINE_JoseDaniel/Blueprints/BP_ThirdPersonCharacter.BP_ThirdPersonCharacter_C|SetScore _asbp_third_person_character (+ (Variables|/Game/CAPITAINE_JoseDaniel/Blueprints/BP_ThirdPersonCharacter.BP_ThirdPersonCharacter_C|GetScore _asbp_third_person_character) (Variables|Default|GetScore%20Value))))
  (Actor|DestroyActor)
  (bind _foundwidgets (Widget|GetAllWidgetsOfClass "/Game/CAPITAINE_JoseDaniel/UI/WBP_Score.WBP_Score_C" true))
  (for _array_element _foundwidgets
    (Variables|/Game/CAPITAINE_JoseDaniel/UI/WBP_Score.WBP_Score_C|SetDisplay%20Text _array_element (Utilities|String|Append "Score : " (Utilities|String|ToString(Integer) _output_get)))))

(fn ConstructionScript)